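; BP_PlayerController is the game's player controller that registers the default input mapping and handles pausing.
; On BeginPlay it adds IMC_Default to the Enhanced Input subsystem.
; When IA_Pause starts, it pauses the game and pushes the CAW_Pause widget onto the main UI stack.
; It then switches to UI-only input focused on that widget, shows the cursor and centres it in the viewport.
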(event Input|EnhancedActionEvents|EnhancedInputActionIA_Pause
  (params (ActionValue :type Boolean) (ElapsedSeconds :type Float%20%28double-precision%29) (TriggeredSeconds :type Float%20%28double-precision%29) (InputAction :type Input%20Action%20Object%20Reference :default "/Game/Input/IA_Pause.IA_Pause"))
  (bind _returnvalue (Viewport|GetViewportSize))
  (bind _self self)
  (bind (_x _y) (Math|Vector2D|BreakVector2D _returnvalue))
  (:Started
    (Game|SetGamePaused true)
    (bind _returnvalue_2 (Class|CommonActivatableWidgetContainerBase|AddWidget (Utilities|ReturnMainstack _self) "/Game/BluePrints/UI/CAW_Pause.CAW_Pause_C"))
    (Input|SetInputModeUIOnly _self _returnvalue_2 "DoNotLock" true)
    (Variables|Default|SetbShowMouseCursor true)
    (Class|PlayerController|SetMouseLocation (Math|Float|Truncate (/ _x 2.0)) (Math|Float|Truncate (/ _y 2.0)))))

(event EventBeginPlay
  (Input|AddMappingContext (PlayerController|LocalPlayerSubsystems|GetEnhancedInputLocalPlayerSubsystem) "/Game/Input/IMC_Default.IMC_Default" 0 "(bIgnoreAllPressedKeysUntilRelease=True,bForceImmediately=False,bNotifyUserSettings=False)"))

(fn ConstructionScript)