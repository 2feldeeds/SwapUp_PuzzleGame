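; Player character with movement, sensitivity-scaled look, jumping, footstep audio, interaction and physics-based object carrying.
; Look, move and jump input refresh a line trace that caches BPI_Interact targets and drives an MPC crosshair animation near DCubes.
; A per-tick trace feeds a toggled PhysicsHandle grab, with gameplay tags tracking the held state.
; A sphere trace underfoot blocks interacting with or grabbing the object being stood on.
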(event Custom|InteractCheck
  (bind _guntrace (Variables|Default|GetGunTrace))
  (bind _returnvalue (Transformation|GetWorldLocation _guntrace))
  ;[0.03044 0.1139 0.15 0.5] Interacting Trace
  (bind (_outhit _returnvalue_2) (Collision|LineTraceByChannel _returnvalue (+ _returnvalue (* (Math|Vector|GetForwardVector _guntrace) (Variables|Default|GetInteractRange))) "TraceTypeQuery1" false 0 "ForDuration" true "(R=1.000000,G=0.000000,B=0.000000,A=1.000000)" "(R=0.000000,G=1.000000,B=0.000000,A=1.000000)" 0.1))
  (if _returnvalue_2
    (Variables|Default|SetHitLocation (- (.Location (Collision|BreakHitResult _outhit)) (* (Math|Vector|GetForwardVector (Variables|Default|GetGunTrace)) 5e+01)))
    (bind _isinteractable (Class|BPIInteract|ReturnInteractStatus(Message) (.HitActor (Collision|BreakHitResult _outhit))))
    (if (and _isinteractable (Utilities|DoesObjectImplementInterface (.HitActor (Collision|BreakHitResult _outhit)) "/Game/BluePrints/Interface/BPI_Interact.BPI_Interact_C"))
      (Variables|Default|SetCurrentInteractable (.HitActor (Collision|BreakHitResult _outhit)))
      (Variables|Default|SetIsLookingAtActor true)
      (else
        (Variables|Default|SetIsLookingAtActor false)
        (bind _hasactivetag_ (Class|BPIGameplayTagFunctions|HasActiveGameplayTag(Message) (Variables|Default|GetCurrentInteractable) "(TagName=\"Dcube.Selected\")" false))
        (if (not _hasactivetag_)
          (Variables|Default|SetCurrentInteractable 0))))))

(event Custom|Crosshair
  ;[0.15 0.15 0.15 0.5] CrossHair
  (bind _outactors (Actor|GetAllActorsOfClass "/Game/BluePrints/World/BP_DCube.BP_DCube_C"))
  (if (and (<= (.Distance (Actor|FindNearestActor (Transformation|GetActorLocation) _outactors)) 3e+02) (Variables|Default|GetIsLookingAtActor))
    (bind _value (Timeline|CrossHair%20Timeline Play)
      (:Update
        (Rendering|Material|SetScalarParameterValue "/Game/Materials/UI/MPC_UI.MPC_UI" "Crosshair" _value :!class /Script/Engine.KismetMaterialLibrary)))
    (else
      (Timeline|CrossHair%20Timeline Reverse))))

(event Custom|InputUpdate
  (CallFunction|InteractCheck)
  (CallFunction|Crosshair))

(event Input|EnhancedActionEvents|EnhancedInputActionIA_Look
  (params (ActionValue :type Vector%202D%20Structure) (ElapsedSeconds :type Float%20%28double-precision%29) (TriggeredSeconds :type Float%20%28double-precision%29) (InputAction :type Input%20Action%20Object%20Reference :default "/Game/Input/IA_Look.IA_Look"))
  (bind (_x _y) (Math|Vector2D|BreakVector2D ActionValue))
  (bind _savesettingsref (Variables|Default|GetSaveSettingsRef))
  (bind _looksens (Variables|/Game/BluePrints/Core/SettingsSave.SettingsSave_C|GetLookSens _savesettingsref))
  ;[0.15 0 0.0921 0.5] Core Input Actions
  (Pawn|Input|AddControllerYawInput (* _x _looksens))
  (Pawn|Input|AddControllerPitchInput (* _y _looksens))
  (Utilities|FlowControl|Delay 0.1)
  (CallFunction|InputUpdate))

(event Input|EnhancedActionEvents|EnhancedInputActionIA_Move
  (params (ActionValue :type Vector%202D%20Structure) (ElapsedSeconds :type Float%20%28double-precision%29) (TriggeredSeconds :type Float%20%28double-precision%29) (InputAction :type Input%20Action%20Object%20Reference :default "/Game/Input/IA_Move.IA_Move"))
  (bind (_x _y) (Math|Vector2D|BreakVector2D ActionValue))
  ;[0.15 0 0.0921 0.5] Core Input Actions
  (Pawn|Input|AddMovementInput (Transformation|GetActorRightVector) _x false)
  (Pawn|Input|AddMovementInput (Transformation|GetActorForwardVector) _y false)
  (CallFunction|InputUpdate))

(event Input|EnhancedActionEvents|EnhancedInputActionIA_Jump
  (params (ActionValue :type Boolean) (ElapsedSeconds :type Float%20%28double-precision%29) (TriggeredSeconds :type Float%20%28double-precision%29) (InputAction :type Input%20Action%20Object%20Reference :default "/Game/Input/IA_Jump.IA_Jump"))
  ;[0.15 0 0.0921 0.5] Core Input Actions
  (:Started
    (if (not (Variables|Default|GetHoldObject))
      (Character|Jump)
      (Audio|PlaySound2D "/Game/Audio/World/Jump.Jump" 1.0 1.0 0.0 0 0)
      (Utilities|CheckBelow (Variables|Default|GetCurrentInteractable))
      (CallFunction|InputUpdate :!label _label)))
  (:Completed
    (Character|StopJumping)
    (goto _label)))

(event Input|EnhancedActionEvents|EnhancedInputActionIA_Interact
  (params (ActionValue :type Boolean) (ElapsedSeconds :type Float%20%28double-precision%29) (TriggeredSeconds :type Float%20%28double-precision%29) (InputAction :type Input%20Action%20Object%20Reference :default "/Game/Input/IA_Interact.IA_Interact"))
  ;[0.15 0.15 0.15 0.5] Interact
  (:Started
    (bind _currentinteractable (Variables|Default|GetCurrentInteractable)
      (:then
        (bind _smthbelow (Utilities|CheckBelow _currentinteractable))
        (if _smthbelow
          (Class|BPIInteract|Interact(Message) (Variables|Default|GetCurrentInteractable) self (Variables|Default|GetHitLocation))))
      (:else))))

(event Input|EnhancedActionEvents|EnhancedInputActionIA_Hold
  (params (ActionValue :type Vector%202D%20Structure) (ElapsedSeconds :type Float%20%28double-precision%29) (TriggeredSeconds :type Float%20%28double-precision%29) (InputAction :type Input%20Action%20Object%20Reference :default "/Game/Input/IA_Hold.IA_Hold"))
  ;[0.15 0.15 0.15 0.5] Hold Item
  (:Started
    (Utilities|FlowControl|FlipFlop
      (:A
        (bind _currentinteractable (Variables|Default|GetCurrentInteractable)
          (:then
            (bind _smthbelow (Utilities|CheckBelow _currentinteractable))
            (if _smthbelow
              (CallFunction|GrabObject)
              (Variables|Default|SetHoldObject true)
              (Default|CallSuccefullInteractDispatcher)))
          (:else)))
      (:B
        (CallFunction|ReleaseObject)
        (Variables|Default|SetHoldObject false)))))

(event EventBeginPlay
  (Components|Timeline|SetPlayRate (Variables|Default|GetCrossHair%20TimeLine) 3.0) ; Speed of the CrossHair Animation
  (Rendering|SetCastShadow (Variables|Default|GetSwapUpGun) false)
  (bind _asbp_game_instance (Utilities|Casting|CastToBP_GameInstance (Game|GetGameInstance)))
  (Variables|Default|SetSaveSettingsRef (Variables|/Game/BluePrints/Core/BP_GameInstance.BP_GameInstance_C|GetSaveSettings _asbp_game_instance))
  (Audio|Components|Audio|Play (Variables|Default|GetFootstep)))

(event EventAddGameplayTags
  (params (GameplayTagsToAdd :type Gameplay%20Tag%20Container%20Structure))
  (CallFunction|AddGameplayTag (Variables|Default|GetGameplayTags) GameplayTagsToAdd))

(event EventTick
  (params (DeltaSeconds :type Float%20%28single-precision%29))
  (bind _guntrace (Variables|Default|GetGunTrace))
  ;[0.15 0.15 0.15 0.5] Trace To Hold Item
  (CallFunction|TraceFunction)
  (if (GameplayTags|HasTag (Variables|Default|GetGameplayTags) "(TagName=\"Player.GrabbedObject\")")
    (Physics|Components|PhysicsHandle|SetTargetLocation (Variables|Default|GetPhysicsHandle) (+ (Transformation|GetWorldLocation _guntrace) (* (Math|Vector|GetForwardVector _guntrace) 1.7e+02)))))

(event EventRemoveGameplayTags
  (params (GamplayTagsToRemove :type Gameplay%20Tag%20Container%20Structure))
  (CallFunction|RemoveGameplayTags GamplayTagsToRemove (Variables|Default|GetGameplayTags)))

(fn ConstructionScript)

(fn TraceFunction
  (bind _guntrace (Variables|Default|GetGunTrace))
  (bind _returnvalue (Transformation|GetWorldLocation _guntrace))
  (bind _outhit (Collision|LineTraceByChannel _returnvalue (+ _returnvalue (* (Math|Vector|GetForwardVector _guntrace) 3e+02)) "TraceTypeQuery1" false 0 "ForOneFrame"))
  (Variables|Default|SetOut%20Hit _outhit)
  (return))

(fn GrabObject
  (bind _out_hit (Variables|Default|GetOut%20Hit))
  (bind _out_hit_2 (Variables|Default|GetOut%20Hit))
  (if (Utilities|IsValid (.hitactor _out_hit))
    (bind _smthbelow (Utilities|CheckBelow (.hitactor _out_hit)))
    (if _smthbelow
      (Class|PrimitiveComponent|SetUseCCD (.hitcomponent _out_hit_2) true "None")
      (Class|PhysicsHandleComponent|GrabComponentatLocation (Variables|Default|GetPhysicsHandle) (.hitcomponent _out_hit_2) "None" (Transformation|GetWorldLocation (.hitcomponent _out_hit_2)))
      (Variables|Default|SetGrabbedActor (.hitactor _out_hit_2))
      (GameplayTags|AddGameplayTag (Variables|Default|GetGameplayTags) "(TagName=\"Player.GrabbedObject\")" :!class /Script/GameplayTags.BlueprintGameplayTagLibrary)
      (return)
      (else
        (return)))))

(fn ReleaseObject
  (bind _gameplaytags (Variables|Default|GetGameplayTags))
  (bind _physicshandle (Variables|Default|GetPhysicsHandle))
  (bind _returnvalue (Class|PhysicsHandleComponent|GetGrabbedComponent _physicshandle))
  (if (GameplayTags|HasTag _gameplaytags "(TagName=\"Player.GrabbedObject\")")
    (Utilities|IsValid _returnvalue :!label _label
      (:Is%20Valid
        (Class|PrimitiveComponent|SetUseCCD _returnvalue false "None")
        (Physics|Components|PhysicsHandle|ReleaseComponent _physicshandle)
        (GameplayTags|RemoveGameplayTag _gameplaytags "(TagName=\"Player.GrabbedObject\")" :!class /Script/GameplayTags.BlueprintGameplayTagLibrary)
        (if (not true)
          (Variables|Default|SetGrabbedActor 0)
          (return)))
      (:Is%20Not%20Valid
        (goto _label)))))

(fn HasActiveGameplayTag
  (params (Tag :type Gameplay%20Tag%20Structure) (LookForExactMatch? :type Boolean))
  (bind _hasactivetag_ (CallFunction|HasActiveGameplayTag (Variables|Default|GetGameplayTags) Tag LookForExactMatch?))
  (return _hasactivetag_))