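; BP_Moveable is an interactable world object that toggles its MoveScene component between a starting and a target transform.
; BeginPlay caches the starting relative transform.
; Each Interact flips a FlipFlop to pick the destination, then MoveComponentTo eases location and rotation there along the shortest rotation path.
; IsInteractable is cleared during the move and restored afterwards, with ReturnInteractStatus exposing it.
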(event EventInteract
  (params (Sender :type Actor%20Object%20Reference))
  (Variables|Default|SetIs%20Interactable false)
  (bind _isa (Utilities|FlowControl|FlipFlop)
    (:A
      _)
    (:B
      _))
  (Components|MoveComponentTo (Variables|Default|GetMoveScene) (.Location (Math|Transform|BreakTransform (Math|Transform|SelectTransform (Variables|Default|GetTargetTransform) (Variables|Default|GetStartTransform) _isa))) (.Rotation (Math|Transform|BreakTransform (Math|Transform|SelectTransform (Variables|Default|GetTargetTransform) (Variables|Default|GetStartTransform) _isa))) true true 1.0 true)
  (Variables|Default|SetIs%20Interactable true))

(event EventBeginPlay
  (Variables|Default|SetStartTransform (Transformation|GetRelativeTransform (Variables|Default|GetMoveScene))))

(fn ConstructionScript)

(fn ReturnInteractStatus
  (return (Variables|Default|GetIs%20Interactable)))