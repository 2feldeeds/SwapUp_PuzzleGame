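; Collectible world actor that highlights its mesh with an outline when it receives an Interact event.
; BeginPlay clears the mesh overlay material, and Interact applies the outline material as an overlay.
; ReturnInteractStatus reports the IsInteractable flag to callers.
; Nodes that disable shadow and collision or set IsInteractable are unconnected, so the actor has no pickup or removal behavior.
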(event EventInteract
  (params (Sender :type Actor%20Object%20Reference))
  (Rendering|Material|SetOverlayMaterial (Variables|Default|GetMesh) "/Game/Materials/World/MI_Outline.MI_Outline" :!class /Script/Engine.MeshComponent))

(event EventBeginPlay
  (Rendering|Material|SetOverlayMaterial (Variables|Default|GetMesh) 0 :!class /Script/Engine.MeshComponent))

(fn ConstructionScript)

(fn ReturnInteractStatus
  (return (Variables|Default|GetIs%20Interactable)))