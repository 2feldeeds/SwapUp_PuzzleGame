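; BP_PressurePlateD is a pressure plate that responds only to actors carrying the Dcube gameplay tag.
; Overlapping its ButtonTrigger plays a double-speed Timeline that lerps the Button's relative Z downward, and ending the overlap reverses it.
; The tag is checked through a gameplay tag interface message, without casting.
; The file shows only the button movement, with no signal to other actors.
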(event OnComponentBeginOverlap(ButtonTrigger)
  (params (OverlappedComponent :type Primitive%20Component%20Object%20Reference) (OtherActor :type Actor%20Object%20Reference) (OtherComp :type Primitive%20Component%20Object%20Reference) (OtherBodyIndex :type Integer) (bFromSweep :type Boolean) (SweepResult :type Hit%20Result%20Structure%20%28by%20ref%29))
  (bind _hasactivetag_ (Class|BPIGameplayTagFunctions|HasActiveGameplayTag(Message) OtherActor "(TagName=\"Dcube\")" false))
  (if _hasactivetag_
    (bind _buton (Timeline|Timeline Play)
      (:Update
        (Transformation|SetRelativeLocation (Variables|Default|GetButton) (Math|Vector|MakeVector 0.0 0.0 (Math|Float|Lerp 3e+01 13.0 _buton)) false false)))))

(event OnComponentEndOverlap(ButtonTrigger)
  (params (OverlappedComponent :type Primitive%20Component%20Object%20Reference) (OtherActor :type Actor%20Object%20Reference) (OtherComp :type Primitive%20Component%20Object%20Reference) (OtherBodyIndex :type Integer))
  (bind _hasactivetag_ (Class|BPIGameplayTagFunctions|HasActiveGameplayTag(Message) OtherActor "(TagName=\"Dcube\")" false))
  (if _hasactivetag_
    (bind _buton (Timeline|Timeline Reverse)
      (:Update
        (Transformation|SetRelativeLocation (Variables|Default|GetButton) (Math|Vector|MakeVector 0.0 0.0 (Math|Float|Lerp 3e+01 13.0 _buton)) false false)))))

(event EventBeginPlay
  (Components|Timeline|SetPlayRate (Variables|Default|GetTimeline) 2.0))

(fn ConstructionScript)