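; BP_Platform is a world actor whose platform component moves up and down continuously as soon as play begins.
; A slowed-down timeline scales its track value into the component's relative Z, while X stays at a fixed offset.
; When the timeline finishes, its direction selects either ReversePlatform or StartPlatform, so the motion ping-pongs endlessly.
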(event Custom|ReversePlatform
  (bind (_direction _newtrack_0) (Timeline|Timeline Reverse)
    (:Update
      (Transformation|SetRelativeLocation (Variables|Default|GetPlatform) (Math|Vector|MakeVector 5e+01 0.0 (* _newtrack_0 5.1e+02)) false false))
    (:Finished
      (switch Utilities|FlowControl|Switch|SwitchonETimelineDirection _direction
        (:Forward
          (CallFunction|ReversePlatform))
        (:Backward
          (CallFunction|StartPlatform))))))

(event Custom|StartPlatform
  (bind (_direction _newtrack_0) (Timeline|Timeline Play)
    (:Update
      (Transformation|SetRelativeLocation (Variables|Default|GetPlatform) (Math|Vector|MakeVector 5e+01 0.0 (* _newtrack_0 5.1e+02)) false false))
    (:Finished
      (switch Utilities|FlowControl|Switch|SwitchonETimelineDirection _direction
        (:Forward
          (CallFunction|ReversePlatform))
        (:Backward
          (CallFunction|StartPlatform))))))

(event EventBeginPlay
  (Components|Timeline|SetPlayRate (Variables|Default|GetTimeline) 0.2)
  (CallFunction|StartPlatform))

(fn ConstructionScript)