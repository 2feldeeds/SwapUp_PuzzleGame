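; BP_PlatformSideWays is a moving platform that slides back and forth along its local Y axis.
; A timeline, slowed at BeginPlay, drives a Lerp that sets the Platform component's relative location.
; When the timeline finishes, its direction selects StartPlatform or ReversePlatform, producing endless ping-pong motion once started.
; BeginPlay calls the parent implementation but does not call StartPlatform itself.
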(event EventBeginPlay
  (Components|Timeline|SetPlayRate (Variables|Default|GetTimeline_0) 0.2)
  (|CallParentFunction))

(event Collision|EventActorBeginOverlap
  (params (OtherActor :type Actor%20Object%20Reference)))

(event EventTick
  (params (DeltaSeconds :type Float%20%28single-precision%29)))

(event EventStartPlatform
  (bind (_direction _newtrack_0) (Timeline|Timeline_0 Play)
    (:Update
      (Transformation|SetRelativeLocation (Variables|Default|GetPlatform) (Math|Vector|MakeVector 5e+01 (Math|Float|Lerp -3.5e+02 3.5e+02 _newtrack_0) 0.0) false false))
    (:Finished
      (switch Utilities|FlowControl|Switch|SwitchonETimelineDirection _direction
        (:Forward
          (CallFunction|ReversePlatform))
        (:Backward
          (CallFunction|StartPlatform))))))

(event EventReversePlatform
  (bind (_direction _newtrack_0) (Timeline|Timeline_0 Reverse)
    (:Update
      (Transformation|SetRelativeLocation (Variables|Default|GetPlatform) (Math|Vector|MakeVector 5e+01 (Math|Float|Lerp -3.5e+02 3.5e+02 _newtrack_0) 0.0) false false))
    (:Finished
      (switch Utilities|FlowControl|Switch|SwitchonETimelineDirection _direction
        (:Forward
          (CallFunction|ReversePlatform))
        (:Backward
          (CallFunction|StartPlatform))))))

(fn ConstructionScript
  (|CallParentFunction))