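; BP_Button is an interactable world button that can be pressed when the interacting actor is close enough.
; On Interact it prints the Sender's distance from the Base and, within range, plays a timeline that drives the Button's relative Z location.
; The timeline update sets IsPressed and clears IsInteractable, which ReturnInteractStatus exposes; nothing in this Blueprint resets either flag.
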(event EventInteract
  (params (Sender :type Actor%20Object%20Reference) (CurrentActor :type Actor%20Object%20Reference) (Transform :type Vector :default "0, 0, 0"))
  (bind _array (Utilities|Array|MakeArray Sender))
  (bind _base (Variables|Default|GetBase))
  (bind _returnvalue (Transformation|GetWorldLocation _base))
  (bind _distance (Actor|FindNearestActor _returnvalue _array))
  (Development|PrintString (Utilities|String|ToString(Float) _distance))
  (if (<= _distance 2e+02)
    (bind _buton (Timeline|Timeline Play)
      (:Update
        (Transformation|SetRelativeLocation (Variables|Default|GetButton) (Math|Vector|MakeVector 0.0 0.0 (* _buton 1e+02)) false false)
        (Variables|Default|SetIs%20Interactable false)
        (Variables|Default|SetIsPressed true)))))

(fn ConstructionScript)

(fn ReturnInteractStatus
  (return (Variables|Default|GetIs%20Interactable)))