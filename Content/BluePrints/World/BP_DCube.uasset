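; BP_DCube is an interactable cube that a BP_Character selects and then places in the world.
; Each Interact call flips between selecting, with an outline overlay and Dcube.Selected tag, and releasing.
; Release restores the BlackWorld overlay and base tag, clears the character's CurrentInteractable and teleports the mesh to the passed transform.
; It also exposes its gameplay tag and interactable status through query functions.
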(event EventInteract
  (params (Sender :type Actor%20Object%20Reference) (Transform :type Vector :default "0, 0, 0"))
  (bind _mesh (Variables|Default|GetMesh))
  (bind _asbp_character (Utilities|Casting|CastToBP_Character Sender))
  (Utilities|FlowControl|FlipFlop
    (:A
      (Rendering|Material|SetOverlayMaterial _mesh "/Game/Materials/World/MI_Outline.MI_Outline" :!class /Script/Engine.MeshComponent)
      (Variables|Default|SetDCubeTag "(GameplayTags=((TagName=\"Dcube.Selected\")))"))
    (:B
      (Rendering|Material|SetOverlayMaterial _mesh "/Game/Materials/World/MI_BlackWorld.MI_BlackWorld" :!class /Script/Engine.MeshComponent)
      (Variables|/Game/BluePrints/Core/BP_Character.BP_Character_C|SetCurrentInteractable _asbp_character 0)
      (Variables|Default|SetDCubeTag "(GameplayTags=((TagName=\"Dcube\")))")
      (Transformation|SetWorldTransform _mesh (Math|Transform|MakeTransform Transform "0, 0, 0" "1.000000,1.000000,1.000000") false true))))

(fn ConstructionScript)

(fn HasActiveGameplayTag
  (params (Tag :type Gameplay%20Tag%20Structure) (LookForExactMatch? :type Boolean))
  (bind _hasactivetag_ (CallFunction|HasActiveGameplayTag (Variables|Default|GetDCubeTag) Tag LookForExactMatch?))
  (return _hasactivetag_))

(fn ReturnInteractStatus
  (return (Variables|Default|GetIs%20Interactable)))